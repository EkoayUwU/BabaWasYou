(fn `CheckIfLinked`
  (returns (Operator :type "/Game/BabaWasYou/Core/Data/E_Operators Enum") (Rule :type "/Game/BabaWasYou/Core/Data/E_Rules Enum"))
  (bind _returnvalue (`self.K2_GetActorLocation`))
  (bind (_outhit _returnvalue_2) (`KismetSystemLibrary.LineTraceSingleForObjects` _returnvalue (+ _returnvalue (-100.0 0.0 0.0)) (`|MakeArray` "ObjectTypeQuery1" "ObjectTypeQuery2" :!type "EObjectTypeQuery Enum")))
  (if _returnvalue_2
    (bind _asbp_rules (cast `/Game/BabaWasYou/Core/Characters/BP_Rules` (`.HitActor` (`GameplayStatics.BreakHitResult` _outhit)))
      (:`then`
        (bind _rule (`/Game/BabaWasYou/Core/Characters/BP_Rules.CheckIfLinked` _asbp_rules))
        (return (`self.Operator`) _rule))
      (:`CastFailed`
        _)))
  (return (`self.Operator`) "NewEnumerator3"))

(fn `UserConstructionScript`
  (`parent.UserConstructionScript`))