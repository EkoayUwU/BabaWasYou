(event `InitInputReceiveRef`
  (params (IR_Ref :type "/Game/BabaWasYou/Core/Characters/BP_InputsReceiver Object Reference"))
  (set `self.IR Ref` IR_Ref))

(fn `CheckIfCanMove`
  (params (Direction :type "/Game/BabaWasYou/Core/Data/E_Sides Enum" :default "NewEnumerator0"))
  (returns (ReturnValue :type Boolean))
  (locals (L_CanMove :type Boolean))
  (bind _returnvalue (`self.K2_GetActorLocation`))
  (bind _array (`|MakeArray` "ObjectTypeQuery1" "ObjectTypeQuery2" :!type "EObjectTypeQuery Enum"))
  (switch `/Game/BabaWasYou/Core/Data/E_Sides` Direction
    (:`NewEnumerator0`
      (bind (_outhit _returnvalue_2) (`KismetSystemLibrary.LineTraceSingleForObjects` _returnvalue (+ _returnvalue (100.0 0.0 0.0)) _array))
      (if _returnvalue_2
        (bind (_bblockinghit _binitialoverlap _time _distance _location _impactpoint _normal _impactnormal _physmat _hitactor) (`GameplayStatics.BreakHitResult` _outhit))
        (bind _asbp_actor_pc (cast `/Game/BabaWasYou/Core/Characters/BP_Actor_PC` _hitactor)
          (:`then`
            (bind _returnvalue_3 (message `GameplayTagAssetInterface.HasMatchingGameplayTag` _hitactor (struct :`TagName` "Rules.STOP")))
            (bind _returnvalue_4 (message `GameplayTagAssetInterface.HasMatchingGameplayTag` _hitactor (struct :`TagName` "Rules.YOU")))
            (if (not (or _returnvalue_3 _returnvalue_4))
              (bind _bmoved (`self.MoveUp` _asbp_actor_pc))
              (return _bmoved)
              (else
                (return (and (not _returnvalue_3) (not (`self.ActorHasTag` _hitactor "STOP")))))))
          (:`CastFailed`
            (return false)))
        (else
          (return true))))
    (:`NewEnumerator1`
      (bind (_outhit_2 _returnvalue_5) (`KismetSystemLibrary.LineTraceSingleForObjects` _returnvalue (+ _returnvalue (-100.0 0.0 0.0)) _array))
      (if _returnvalue_5
        (bind (_bblockinghit_2 _binitialoverlap_2 _time_2 _distance_2 _location_2 _impactpoint_2 _normal_2 _impactnormal_2 _physmat_2 _hitactor_2) (`GameplayStatics.BreakHitResult` _outhit_2))
        (bind _asbp_actor_pc_2 (cast `/Game/BabaWasYou/Core/Characters/BP_Actor_PC` _hitactor_2)
          (:`then`
            (bind _returnvalue_6 (message `GameplayTagAssetInterface.HasMatchingGameplayTag` _hitactor_2 (struct :`TagName` "Rules.STOP")))
            (bind _returnvalue_7 (message `GameplayTagAssetInterface.HasMatchingGameplayTag` _hitactor_2 (struct :`TagName` "Rules.YOU")))
            (if (not (or _returnvalue_6 _returnvalue_7))
              (bind _bmoved_2 (`self.MoveDown` _asbp_actor_pc_2))
              (return _bmoved_2)
              (else
                (return (and (not _returnvalue_6) (not (`self.ActorHasTag` _hitactor_2 "STOP")))))))
          (:`CastFailed`
            (return false)))
        (else
          (return true))))
    (:`NewEnumerator2`
      (bind (_outhit_3 _returnvalue_8) (`KismetSystemLibrary.LineTraceSingleForObjects` _returnvalue (+ _returnvalue (-0.0 -100.0 0.0)) _array))
      (if _returnvalue_8
        (bind (_bblockinghit_3 _binitialoverlap_3 _time_3 _distance_3 _location_3 _impactpoint_3 _normal_3 _impactnormal_3 _physmat_3 _hitactor_3) (`GameplayStatics.BreakHitResult` _outhit_3))
        (bind _asbp_actor_pc_3 (cast `/Game/BabaWasYou/Core/Characters/BP_Actor_PC` _hitactor_3)
          (:`then`
            (bind _returnvalue_9 (message `GameplayTagAssetInterface.HasMatchingGameplayTag` _hitactor_3 (struct :`TagName` "Rules.STOP")))
            (bind _returnvalue_10 (message `GameplayTagAssetInterface.HasMatchingGameplayTag` _hitactor_3 (struct :`TagName` "Rules.YOU")))
            (if (not (or _returnvalue_9 _returnvalue_10))
              (bind _bmoved_3 (`self.MoveLeft` _asbp_actor_pc_3))
              (return _bmoved_3)
              (else
                (return (and (not _returnvalue_9) (not (`self.ActorHasTag` _hitactor_3 "STOP")))))))
          (:`CastFailed`
            (return false)))
        (else
          (return true))))
    (:`NewEnumerator3`
      (bind (_outhit_4 _returnvalue_11) (`KismetSystemLibrary.LineTraceSingleForObjects` _returnvalue (+ _returnvalue (0.0 100.0 0.0)) _array))
      (if _returnvalue_11
        (bind (_bblockinghit_4 _binitialoverlap_4 _time_4 _distance_4 _location_4 _impactpoint_4 _normal_4 _impactnormal_4 _physmat_4 _hitactor_4) (`GameplayStatics.BreakHitResult` _outhit_4))
        (bind _asbp_actor_pc_4 (cast `/Game/BabaWasYou/Core/Characters/BP_Actor_PC` _hitactor_4)
          (:`then`
            (bind _returnvalue_12 (message `GameplayTagAssetInterface.HasMatchingGameplayTag` _hitactor_4 (struct :`TagName` "Rules.STOP")))
            (bind _returnvalue_13 (message `GameplayTagAssetInterface.HasMatchingGameplayTag` _hitactor_4 (struct :`TagName` "Rules.YOU")))
            (if (not (or _returnvalue_12 _returnvalue_13))
              (bind _bmoved_4 (`self.MoveRight` _asbp_actor_pc_4))
              (return _bmoved_4)
              (else
                (return (and (not _returnvalue_12) (not (`self.ActorHasTag` _hitactor_4 "STOP")))))))
          (:`CastFailed`
            (return false)))
        (else
          (return true))))))

(fn `MoveDown`
  (returns (bMoved :type Boolean))
  (bind _returnvalue (`self.CheckIfCanMove` "NewEnumerator1"))
  (if _returnvalue
    (set `self.SideToCheck` "NewEnumerator1")
    (`self.K2_SetActorLocation` (+ (`self.K2_GetActorLocation`) (-100.0 0.0 0.0)))
    (return true)
    (else
      (set `self.SideToCheck` "NewEnumerator1")
      (return false))))

(fn `MoveLeft`
  (returns (bMoved :type Boolean))
  (bind _returnvalue (`self.CheckIfCanMove` "NewEnumerator2"))
  (if _returnvalue
    (set `self.SideToCheck` "NewEnumerator2")
    (`self.K2_SetActorLocation` (+ (`self.K2_GetActorLocation`) (0.0 -100.0 0.0)))
    (return true)
    (else
      (set `self.SideToCheck` "NewEnumerator2")
      (return false))))

(fn `MoveRight`
  (returns (bMoved :type Boolean))
  (bind _returnvalue (`self.CheckIfCanMove` "NewEnumerator3"))
  (if _returnvalue
    (set `self.SideToCheck` "NewEnumerator3")
    (`self.K2_SetActorLocation` (+ (`self.K2_GetActorLocation`) (0.0 100.0 0.0)))
    (return true)
    (else
      (set `self.SideToCheck` "NewEnumerator3")
      (return false))))

(fn `MoveUp`
  (returns (bMoved :type Boolean))
  (bind _returnvalue (`self.CheckIfCanMove` "NewEnumerator0"))
  (if _returnvalue
    (set `self.SideToCheck` "NewEnumerator0")
    (`self.K2_SetActorLocation` (+ (`self.K2_GetActorLocation`) (100.0 0.0 0.0)))
    (return true)
    (else
      (set `self.SideToCheck` "NewEnumerator0")
      (return false))))

(fn `UserConstructionScript`
  (`PaperFlipbookComponent.SetFlipbook` (`self.PaperFlipbook`) (`self.FlipBook`)))