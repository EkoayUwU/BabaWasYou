(fn `CheckIfLinked`
  (bind _returnvalue (`self.K2_GetActorLocation`))
  (bind _returnvalue_2 (`self.K2_GetActorLocation`))
  (bind (_outhit _returnvalue_3) (`KismetSystemLibrary.LineTraceSingleForObjects` _returnvalue_2 (+ _returnvalue_2 (-100.0 0.0 0.0)) (`|MakeArray` "ObjectTypeQuery1" "ObjectTypeQuery2" :!type "EObjectTypeQuery Enum")))
  (if _returnvalue_3
    (bind _asbp_operator (cast `/Game/BabaWasYou/Core/Characters/BP_Operator` (`.HitActor` (`GameplayStatics.BreakHitResult` _outhit)))
      (:`then`
        (bind (_operator _rule) (`/Game/BabaWasYou/Core/Characters/BP_Operator.CheckIfLinked` _asbp_operator))
        (bind _output_get (set `self.SentenceStrucure` (make `/Game/BabaWasYou/Core/Characters/S_LinkedList` (`self.Word`) _operator _rule)))
        (`/Game/BabaWasYou/Core/Characters/BP_InputsReceiver.ShouldDoChanges` (`self.IR Ref`) _output_get))
      (:`CastFailed`
        (bind _output_get_2 (set `self.SentenceStrucure` (make `/Game/BabaWasYou/Core/Characters/S_LinkedList` (`self.Word`) "NewEnumerator3" "NewEnumerator3")))
        (`/Game/BabaWasYou/Core/Characters/BP_InputsReceiver.ShouldDoChanges` (`self.IR Ref`) _output_get_2)))
    (else
      (bind (_outhit_2 _returnvalue_4) (`KismetSystemLibrary.LineTraceSingleForObjects` _returnvalue (+ _returnvalue (0.0 100.0 0.0)) (`|MakeArray` "ObjectTypeQuery1" "ObjectTypeQuery2" :!type "EObjectTypeQuery Enum")))
      (if _returnvalue_4
        (bind _asbp_operator_2 (cast `/Game/BabaWasYou/Core/Characters/BP_Operator` (`.HitActor` (`GameplayStatics.BreakHitResult` _outhit_2))))
        (bind (_operator_2 _rule_2) (`/Game/BabaWasYou/Core/Characters/BP_Operator.CheckIfLinked` _asbp_operator_2))
        (bind _output_get_3 (set `self.SentenceStrucure` (make `/Game/BabaWasYou/Core/Characters/S_LinkedList` (`self.Word`) _operator_2 _rule_2)))
        (`/Game/BabaWasYou/Core/Characters/BP_InputsReceiver.ShouldDoChanges` (`self.IR Ref`) _output_get_3)
        (else
          (bind _output_get_4 (set `self.SentenceStrucure` (make `/Game/BabaWasYou/Core/Characters/S_LinkedList` (`self.Word`) "NewEnumerator3" "NewEnumerator3")))
          (`/Game/BabaWasYou/Core/Characters/BP_InputsReceiver.ShouldDoChanges` (`self.IR Ref`) _output_get_4))))))

(fn `UserConstructionScript`
  (`parent.UserConstructionScript`)
  (set `self.SentenceStrucure` (make `/Game/BabaWasYou/Core/Characters/S_LinkedList` (`self.Word`) "NewEnumerator3" "NewEnumerator3")))