(event `MoveUp`
  (`self.K2_SetActorRelativeLocation` (+ (`self.K2_GetActorLocation`) (0.0 50.0 0.0)) true))

(event `Check`)

(event `MoveDown`
  (`self.K2_SetActorRelativeLocation` (+ (`self.K2_GetActorLocation`) (0.0 -50.0 0.0)) true))

(event `MoveLeft`
  (`self.K2_SetActorRelativeLocation` (+ (`self.K2_GetActorLocation`) (50.0 0.0 0.0)) true))

(event `MoveRight`
  (`self.K2_SetActorRelativeLocation` (+ (`self.K2_GetActorLocation`) (-50.0 0.0 0.0)) true))

(fn `UserConstructionScript`)