(fn `CheckIfLinked`
  (returns (Rule :type "/Game/BabaWasYou/Core/Data/E_Rules Enum"))
  (bind _returnvalue (`self.K2_GetActorLocation`))
  (bind (_outhit _returnvalue_2) (`KismetSystemLibrary.LineTraceSingleForObjects` _returnvalue (+ _returnvalue (-100.0 0.0 0.0)) (`|MakeArray` "ObjectTypeQuery1" "ObjectTypeQuery2" :!type "EObjectTypeQuery Enum")))
  (if _returnvalue_2
    (bind _asbp_operator (cast `/Game/BabaWasYou/Core/Characters/BP_Operator` (`.HitActor` (`GameplayStatics.BreakHitResult` _outhit))))
    (if (`|EnumEquality` (`/Game/BabaWasYou/Core/Characters/BP_Operator.Operator` _asbp_operator) "NewEnumerator1")
      (`/Game/BabaWasYou/Core/Characters/BP_Operator.CheckIfLinked` _asbp_operator))
    (else
      (return (`self.Rule`)))))

(fn `UserConstructionScript`
  (`parent.UserConstructionScript`))